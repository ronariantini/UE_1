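; PushButton4_BP is a toggle push button for a panel, with a Box trigger and a Cylinder mesh.
; An overlap by BP_FirstPersonCharacter, or any hit on the Box, flips the boolean VarPB1.
; The state swaps the Cylinder material between solid blue and the base material and prints ON or OFF.
; The variable and messages are labeled PB1 despite the asset's PushButton4 name.
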(event OnComponentBeginOverlap(Box)
  (params (OverlappedComponent :type Primitive%20Component%20Object%20Reference) (OtherActor :type Actor%20Object%20Reference) (OtherComp :type Primitive%20Component%20Object%20Reference) (OtherBodyIndex :type Integer) (bFromSweep :type Boolean) (SweepResult :type Hit%20Result%20Structure%20%28by%20ref%29))
  (bind _cylinder (Variables|Default|GetCylinder))
  (Utilities|Casting|CastToBP_FirstPersonCharacter OtherActor)
  (bind _output_get (Variables|Default|SetVar_PB1 (not (Variables|Default|GetVar_PB1))))
  (if _output_get
    (Rendering|Material|SetMaterial _cylinder 0 "/Game/LevelPrototyping/Materials/MI_Solid_Blue.MI_Solid_Blue")
    (Development|PrintString "PB1 ON")
    (else
      (Rendering|Material|SetMaterial _cylinder 0 "/Game/FPWeapon/Materials/BaseMaterial.BaseMaterial")
      (Development|PrintString "PB1 OFF"))))

(event OnComponentHit(Box)
  (params (HitComponent :type Primitive%20Component%20Object%20Reference) (OtherActor :type Actor%20Object%20Reference) (OtherComp :type Primitive%20Component%20Object%20Reference) (NormalImpulse :type Vector :default "0, 0, 0") (Hit :type Hit%20Result%20Structure%20%28by%20ref%29))
  (bind _cylinder (Variables|Default|GetCylinder))
  (bind _output_get (Variables|Default|SetVar_PB1 (not (Variables|Default|GetVar_PB1))))
  (if _output_get
    (Rendering|Material|SetMaterial _cylinder 0 "/Game/LevelPrototyping/Materials/MI_Solid_Blue.MI_Solid_Blue")
    (Development|PrintString "PB1 ON")
    (else
      (Rendering|Material|SetMaterial _cylinder 0 "/Game/FPWeapon/Materials/BaseMaterial.BaseMaterial")
      (Development|PrintString "PB1 OFF"))))

(event EventBeginPlay)

(event Collision|EventActorBeginOverlap
  (params (OtherActor :type Actor%20Object%20Reference)))

(event EventTick
  (params (DeltaSeconds :type Float%20%28single-precision%29)))

(fn ConstructionScript)