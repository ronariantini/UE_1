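; Wall button actor with a Switch component and a Box collision that reacts to being hit.
; BeginPlay caches the switch's relative transform as the off position, derives an on position shifted along Y, and enables input from the first player controller.
; A Box hit prints a debug string and swaps the switch material to steel.
; The cached positions are never applied, and the overlap handlers are empty.
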(event OnComponentBeginOverlap(Box)
  (params (OverlappedComponent :type Primitive%20Component%20Object%20Reference) (OtherActor :type Actor%20Object%20Reference) (OtherComp :type Primitive%20Component%20Object%20Reference) (OtherBodyIndex :type Integer) (bFromSweep :type Boolean) (SweepResult :type Hit%20Result%20Structure%20%28by%20ref%29)))

(event OnComponentHit(Box)
  (params (HitComponent :type Primitive%20Component%20Object%20Reference) (OtherActor :type Actor%20Object%20Reference) (OtherComp :type Primitive%20Component%20Object%20Reference) (NormalImpulse :type Vector :default "0, 0, 0") (Hit :type Hit%20Result%20Structure%20%28by%20ref%29))
  (Development|PrintString "kena")
  (Rendering|Material|SetMaterial (Variables|Default|Getswitch) 0 "/Game/StarterContent/Materials/M_Metal_Steel.M_Metal_Steel"))

(event EventBeginPlay
  (bind _switch (Variables|Default|Getswitch))
  (bind _returnvalue (Transformation|GetRelativeTransform _switch))
  (Variables|Default|Setoff%20position (Math|Transform|MakeTransform (.location _returnvalue) (.rotation _returnvalue) (.scale _returnvalue)))
  (Variables|Default|Seton%20position (Math|Transform|MakeTransform (- (.location _returnvalue) "0,10.000000,0") (.rotation _returnvalue) (.scale _returnvalue)))
  (Input|EnableInput (Game|GetPlayerController 0)))

(event Collision|EventActorBeginOverlap
  (params (OtherActor :type Actor%20Object%20Reference)))

(event EventTick
  (params (DeltaSeconds :type Float%20%28single-precision%29)))

(fn ConstructionScript)