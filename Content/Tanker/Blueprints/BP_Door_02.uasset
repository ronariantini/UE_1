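; BP_Door_02 is an interactive skeletal-mesh door that the player opens and closes with the Interact input.
; It enables input from player controller 0 on BeginPlay, and Box overlap events set OpenClose, which acts as an in-range flag without filtering the overlapping actor.
; While that flag is set, each Interact press passes through a FlipFlop that alternates the non-looping open and close animations.
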(event OnComponentBeginOverlap(Box)
  (params (OverlappedComponent :type Primitive%20Component%20Object%20Reference) (OtherActor :type Actor%20Object%20Reference) (OtherComp :type Primitive%20Component%20Object%20Reference) (OtherBodyIndex :type Integer) (bFromSweep :type Boolean) (SweepResult :type Hit%20Result%20Structure%20%28by%20ref%29))
  (Variables|Default|SetOpen_close true))

(event OnComponentEndOverlap(Box)
  (params (OverlappedComponent :type Primitive%20Component%20Object%20Reference) (OtherActor :type Actor%20Object%20Reference) (OtherComp :type Primitive%20Component%20Object%20Reference) (OtherBodyIndex :type Integer))
  (Variables|Default|SetOpen_close false))

(event Collision|EventActorBeginOverlap
  (params (OtherActor :type Actor%20Object%20Reference)))

(event EventTick
  (params (DeltaSeconds :type Float%20%28single-precision%29)))

(event EventBeginPlay
  (Input|EnableInput (Game|GetPlayerController 0)))

(event Input|ActionEvents|InputActionInteract
  (params (Key :type Key%20Structure))
  (:Pressed
    (if (Variables|Default|GetOpen_close)
      (Utilities|FlowControl|FlipFlop
        (:A
          (Components|Animation|PlayAnimation (Variables|Default|GetSK_Door_02_Anim) "/Game/Tanker/Skeletal_Mesh/SM_Door_02_Anim_Anim_ArmatureDoor_Door_02_Open.SM_Door_02_Anim_Anim_ArmatureDoor_Door_02_Open" false))
        (:B
          (Components|Animation|PlayAnimation (Variables|Default|GetSK_Door_02_Anim) "/Game/Tanker/Skeletal_Mesh/SM_Door_02_Anim_Anim_ArmatureDoor_Door_02_Close.SM_Door_02_Anim_Anim_ArmatureDoor_Door_02_Close" false))))))

(fn ConstructionScript)