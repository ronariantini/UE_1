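; BP_pickup is a collectible actor that the third-person player character picks up by walking into it.
; A box overlap casts the other actor to BP_ThirdPersonCharacter, calls CollectPickup with IncreaseAmount, then destroys the pickup.
; Overlaps from any other actor print the overlapping component's name.
; The construction script prints the sphere's world scale and assigns it the M_Door material.
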(event OnComponentBeginOverlap(Box)
  (params (OverlappedComponent :type Primitive%20Component%20Object%20Reference) (OtherActor :type Actor%20Object%20Reference) (OtherComp :type Primitive%20Component%20Object%20Reference) (OtherBodyIndex :type Integer) (bFromSweep :type Boolean) (SweepResult :type Hit%20Result%20Structure%20%28by%20ref%29))
  (bind _asbp_third_person_character (Utilities|Casting|CastToBP_ThirdPersonCharacter OtherActor)
    (:then
      (Default|CollectPickup _asbp_third_person_character (Variables|Default|GetIncrease%20Amount))
      (Actor|DestroyActor))
    (:CastFailed
      (Development|PrintString (Utilities|GetDisplayName OtherComp)))))

(event EventTick
  (params (DeltaSeconds :type Float%20%28single-precision%29)))

(event EventBeginPlay)

(fn ConstructionScript
  (Development|PrintString (Utilities|String|ToString(Vector) (Transformation|GetWorldScale (Variables|Default|GetSphere))) true true "(R=0.871714,G=1.000000,B=0.318126,A=1.000000)" 5.0)
  (Rendering|Material|SetMaterial (Variables|Default|GetSphere) 0 "/Game/StarterContent/Props/Materials/M_Door.M_Door"))