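; BP_GoalTrigger is a goal volume that decides win or lose when the third-person character overlaps its box.
; It compares the character's CollectedAmount against a required count.
; Enough pickups prints a win message and plays music once through a DoOnce MultiInput.
; Too few prints a loss message, spawns an explosion with sound, then reloads ThirdPersonMap after a short delay.
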(event OnComponentBeginOverlap(Box)
  (params (OverlappedComponent :type Primitive%20Component%20Object%20Reference) (OtherActor :type Actor%20Object%20Reference) (OtherComp :type Primitive%20Component%20Object%20Reference) (OtherBodyIndex :type Integer) (bFromSweep :type Boolean) (SweepResult :type Hit%20Result%20Structure%20%28by%20ref%29))
  (bind _asbp_third_person_character (Utilities|Casting|CastToBP_ThirdPersonCharacter OtherActor))
  (if (>= (Variables|/Game/ThirdPerson/Blueprints/BP_ThirdPersonCharacter.BP_ThirdPersonCharacter_C|GetCollectedAmount _asbp_third_person_character) 3)
    (|DoOnceMultiInput
      (:A%20Out
        (Development|PrintString "You win" true true "(R=0.339187,G=1.000000,B=0.228182,A=1.000000)")
        (Audio|PlaySound2D "/Game/StarterContent/Audio/Starter_Music01.Starter_Music01" 1.0 1.0 0.0 0 0)))
    (else
      (Development|PrintString "You loose" true true "(R=1.000000,G=0.086179,B=0.455176,A=1.000000)")
      (Effects|SpawnEmitteratLocation "/Game/StarterContent/Particles/P_Explosion.P_Explosion" (Transformation|GetWorldLocation (Variables|Default|GetBox)))
      (Audio|PlaySoundatLocation "/Game/StarterContent/Audio/Explosion01.Explosion01" (Transformation|GetWorldLocation (Variables|Default|GetBox)) "0, 0, 0" 1.0 1.0 0.0 0 0 0 0)
      (Utilities|FlowControl|Delay 3.0)
      (Game|OpenLevel(byName) "ThirdPersonMap"))))

(event EventBeginPlay)

(event Collision|EventActorBeginOverlap
  (params (OtherActor :type Actor%20Object%20Reference)))

(event EventTick
  (params (DeltaSeconds :type Float%20%28single-precision%29)))

(fn ConstructionScript)