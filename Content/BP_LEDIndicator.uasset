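; BP_LEDIndicator is an LED light on an electrical panel that shows red when the panel is an objective and green otherwise.
; Shortly after BeginPlay it casts its parent actor to BP_PanelBase, reads PanelIsObjective and calls TurnRed or TurnGreen to swap the Cube's material.
; An unconnected older branch checks ObjectiveBreaker and sets the game instance's objective text, but never runs.
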(event EventBeginPlay
  (Utilities|FlowControl|Delay 0.4)
  (bind _asbp_panel_base (Utilities|Casting|CastToBP_PanelBase (Actor|GetParentActor)))
  (if (Variables|/Game/Levels/Level2/Blueprints/Panels/BP_PanelBase.BP_PanelBase_C|GetPanelIsObjective _asbp_panel_base)
    (CallFunction|TurnRed)
    (else
      (CallFunction|TurnGreen))))

(event Collision|EventActorBeginOverlap
  (params (OtherActor :type Actor%20Object%20Reference)))

(event EventTick
  (params (DeltaSeconds :type Float%20%28single-precision%29)))

(fn ConstructionScript)

(fn TurnRed
  (Rendering|Material|SetMaterial (Variables|Default|GetCube) 0 "/Game/M_LEDIndicator_Red.M_LEDIndicator_Red"))

(fn TurnGreen
  (Rendering|Material|SetMaterial (Variables|Default|GetCube) 0 "/Game/M_LEDIndicator.M_LEDIndicator"))