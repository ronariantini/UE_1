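; BP_PanelBase is a panel Blueprint in Level2 that can flag one of its child breakers as the objective.
; SetRandomObjective gathers BP_Breaker0 actors from its ChildActorComponents into BreakerArray and sets Objective on one.
; The random index range is fixed at zero, so the first entry is always picked, and each breaker's state is printed for debugging.
; The event graph is empty, so nothing here calls the function.
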(event EventBeginPlay)

(event Collision|EventActorBeginOverlap
  (params (OtherActor :type Actor%20Object%20Reference)))

(event EventTick
  (params (DeltaSeconds :type Float%20%28single-precision%29)))

(fn ConstructionScript)

(fn SetRandomObjective
  (bind _breakerarray (Variables|Default|GetBreakerArray))
  (for _array_element (Actor|GetComponentsByClass "/Script/Engine.ChildActorComponent")
    (bind _asbp_breaker_0 (Utilities|Casting|CastToBP_Breaker0 (Variables|/Script/Engine.ChildActorComponent|GetChildActor _array_element)))
    (Utilities|IsValid _asbp_breaker_0
      (:Is%20Valid
        (Utilities|Array|Add (Variables|Default|GetBreakerArray) _asbp_breaker_0))))
  (Variables|/Game/Levels/Level1/Blueprints/BP_Breaker0.BP_Breaker0_C|SetObjective (Utilities|Array|Get(acopy) _breakerarray (Math|Random|RandomIntegerinRange 0 0)) true)
  (for _array_element_2 _breakerarray
    (Development|PrintString (Utilities|String|Append (Utilities|GetDisplayName _array_element_2) (Utilities|String|ToString(Boolean) (Variables|/Game/Levels/Level1/Blueprints/BP_Breaker0.BP_Breaker0_C|GetObjective _array_element_2))) true true "(R=0.000000,G=0.660000,B=1.000000,A=1.000000)" 1e+01)))