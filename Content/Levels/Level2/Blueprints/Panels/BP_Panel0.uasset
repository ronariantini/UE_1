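; BP_Panel0 is a Level 2 panel Blueprint that picks a random objective when play begins.
; On BeginPlay it runs the parent logic, then calls SetRandomObjective, first waiting briefly if the first BreakerArray entry is not yet valid.
; The wait happens only once, with no recheck of the breaker afterward.
; Overlap and Tick events are disabled, and the construction script only calls its parent.
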(event EventBeginPlay
  (|CallParentFunction)
  (Utilities|IsValid (Utilities|Array|Get(acopy) (Variables|Default|GetBreakerArray))
    (:Is%20Valid
      _)
    (:Is%20Not%20Valid
      (Utilities|FlowControl|Delay 1.0)))
  (CallFunction|SetRandomObjective))

(event Collision|EventActorBeginOverlap
  (params (OtherActor :type Actor%20Object%20Reference))
  (|CallParentFunction OtherActor) ; This node is disabled and will not be called.\nDrag off pins to build functionality.
)

(event EventTick
  (params (DeltaSeconds :type Float%20%28single-precision%29))
  (|CallParentFunction DeltaSeconds) ; This node is disabled and will not be called.\nDrag off pins to build functionality.
)

(fn ConstructionScript
  (|CallParentFunction))