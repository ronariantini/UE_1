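; Breaker switch actor for panel 1 in Level 2, toggled between on and off through its Interact Switch function.
; Each toggle rotates the switch mesh, swaps two standby indicator materials and flips a local state flag.
; The new state is written to the Breaker1 flag on MyGameInstance.
; The box overlap and construction graphs are empty.
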(event OnComponentBeginOverlap(Box)
  (params (OverlappedComponent :type Primitive%20Component%20Object%20Reference) (OtherActor :type Actor%20Object%20Reference) (OtherComp :type Primitive%20Component%20Object%20Reference) (OtherBodyIndex :type Integer) (bFromSweep :type Boolean) (SweepResult :type Hit%20Result%20Structure%20%28by%20ref%29)))

(event OnComponentEndOverlap(Box)
  (params (OverlappedComponent :type Primitive%20Component%20Object%20Reference) (OtherActor :type Actor%20Object%20Reference) (OtherComp :type Primitive%20Component%20Object%20Reference) (OtherBodyIndex :type Integer)))

(event Collision|EventActorBeginOverlap
  (params (OtherActor :type Actor%20Object%20Reference)))

(fn ConstructionScript)

(fn InteractSwitch
  (bind _returnvalue (Game|GetGameInstance))
  (bind _cb_st_by_ind_001 (Variables|Default|GetCB_st_by_ind_001))
  (bind _bp_breaker_switch (Variables|Default|GetBP_Breaker_Switch))
  (bind _cb_st_by_ind_ (Variables|Default|GetCB_st_by_ind_))
  (if (Variables|Default|GetVar_Breaker0)
    (Transformation|SetRelativeRotation _bp_breaker_switch "0.000000,0.000000,20.000000" false false)
    (Rendering|Material|SetMaterial _cb_st_by_ind_ 0 "/Game/Levels/Level1/Circuit_Breaker_obj/st-by_off.st-by_off")
    (Rendering|Material|SetMaterial _cb_st_by_ind_001 0 "/Game/Levels/Level1/Circuit_Breaker_obj/st-by_off.st-by_off")
    (Variables|Default|SetVar_Breaker0 false)
    (bind _asmy_game_instance (Utilities|Casting|CastToMyGameInstance _returnvalue))
    (Variables|/Game/MyGameInstance.MyGameInstance_C|SetBreaker1 _asmy_game_instance false)
    (else
      (Transformation|SetRelativeRotation _bp_breaker_switch "0.000000,0.000000,-90.000000" false false)
      (Rendering|Material|SetMaterial _cb_st_by_ind_ 0 "/Game/Levels/Level1/Circuit_Breaker_obj/st-by_on.st-by_on")
      (Rendering|Material|SetMaterial _cb_st_by_ind_001 0 "/Game/Levels/Level1/Circuit_Breaker_obj/st-by_on.st-by_on")
      (Variables|Default|SetVar_Breaker0 true)
      (bind _asmy_game_instance_2 (Utilities|Casting|CastToMyGameInstance _returnvalue))
      (Variables|/Game/MyGameInstance.MyGameInstance_C|SetBreaker1 _asmy_game_instance_2 true))))