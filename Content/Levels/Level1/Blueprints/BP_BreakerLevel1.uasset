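; BP_BreakerLevel1 is an interactable Level 1 breaker that can hide a fault objective.
; InteractSwitch toggles the lever rotation and standby indicator materials.
; Objective breakers also drive the parent BP_PanelLevel1's LED and randomized gauge needle.
; An objective's first interaction reports the fault, and on the last panel it sets the game mode's condition and ends the game instead of toggling.
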(event OnComponentBeginOverlap(Box)
  (params (OverlappedComponent :type Primitive%20Component%20Object%20Reference) (OtherActor :type Actor%20Object%20Reference) (OtherComp :type Primitive%20Component%20Object%20Reference) (OtherBodyIndex :type Integer) (bFromSweep :type Boolean) (SweepResult :type Hit%20Result%20Structure%20%28by%20ref%29)))

(event OnComponentEndOverlap(Box)
  (params (OverlappedComponent :type Primitive%20Component%20Object%20Reference) (OtherActor :type Actor%20Object%20Reference) (OtherComp :type Primitive%20Component%20Object%20Reference) (OtherBodyIndex :type Integer)))

(event Collision|EventActorBeginOverlap
  (params (OtherActor :type Actor%20Object%20Reference)))

(fn ConstructionScript)

(fn InteractSwitch
  (bind _returnvalue (Actor|GetParentActor))
  (bind _bp_breaker_switch (Variables|Default|GetBP_Breaker_Switch))
  (bind _cb_st_by_ind_001 (Variables|Default|GetCB_st_by_ind_001))
  (bind _cb_st_by_ind_ (Variables|Default|GetCB_st_by_ind_))
  (bind _objective (Variables|Default|GetObjective))
  (if (Variables|Default|GetObjective)
    (if (Variables|Default|GetFoundObjective)
      (if (Variables|Default|GetIsOn) :!label _label
        (Transformation|SetRelativeRotation _bp_breaker_switch "0.000000,0.000000,20.000000" false false)
        (Rendering|Material|SetMaterial _cb_st_by_ind_ 0 "/Game/Levels/Level1/Circuit_Breaker_obj/st-by_off.st-by_off")
        (Rendering|Material|SetMaterial _cb_st_by_ind_001 0 "/Game/Levels/Level1/Circuit_Breaker_obj/st-by_off.st-by_off")
        (Variables|Default|SetIsOn false)
        (if _objective
          (bind _asbp_panel_level_1 (Utilities|Casting|CastToBP_PanelLevel1 _returnvalue))
          (Default|TurnGreen (Variables|/Game/Levels/Level1/Blueprints/BP_PanelLevel1.BP_PanelLevel1_C|GetLEDIndicator _asbp_panel_level_1))
          (Default|TurnNeedle (Variables|/Game/Levels/Level1/Blueprints/BP_PanelLevel1.BP_PanelLevel1_C|GetGauge _asbp_panel_level_1) (Math|Random|RandomFloatinRange 0.6 0.9)))
        (else
          (Transformation|SetRelativeRotation _bp_breaker_switch "0.000000,0.000000,-90.000000" false false)
          (Rendering|Material|SetMaterial _cb_st_by_ind_ 0 "/Game/Levels/Level1/Circuit_Breaker_obj/st-by_on.st-by_on")
          (Rendering|Material|SetMaterial _cb_st_by_ind_001 0 "/Game/Levels/Level1/Circuit_Breaker_obj/st-by_on.st-by_on")
          (Variables|Default|SetIsOn true)
          (if _objective
            (bind _asbp_panel_level_1_2 (Utilities|Casting|CastToBP_PanelLevel1 _returnvalue))
            (Default|TurnRed (Variables|/Game/Levels/Level1/Blueprints/BP_PanelLevel1.BP_PanelLevel1_C|GetLEDIndicator _asbp_panel_level_1_2))
            (Default|TurnNeedle (Variables|/Game/Levels/Level1/Blueprints/BP_PanelLevel1.BP_PanelLevel1_C|GetGauge _asbp_panel_level_1_2) (Math|Random|RandomFloatinRange 0.1 0.2)))))
      (else
        (Variables|Default|SetFoundObjective true)
        (Development|PrintString (Utilities|String|Append "Fault found in " (Utilities|GetDisplayName (Actor|GetParentActor))))
        (bind _asbp_panel_level_1_3 (Utilities|Casting|CastToBP_PanelLevel1 (Actor|GetParentActor)))
        (if (Variables|/Game/Levels/Level1/Blueprints/BP_PanelLevel1.BP_PanelLevel1_C|GetIsLast _asbp_panel_level_1_3)
          (Development|PrintString "Root fault is found")
          (bind _asbp_first_person_game_mode (Utilities|Casting|CastToBP_FirstPersonGameMode (Game|GetGameMode)))
          (Variables|/Game/Levels/Panel/Blueprints/BP_FirstPersonGameMode.BP_FirstPersonGameMode_C|SetGameCondition _asbp_first_person_game_mode true)
          (Default|EndGame _asbp_first_person_game_mode)
          (else
            (goto _label)))))
    (else
      (goto _label))))