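; Level 1 door actor that toggles open and closed and highlights itself when something overlaps its Box trigger.
; InteractDoor flips IsOpened and plays the matching one-shot animation on the skeletal mesh; nothing in this Blueprint calls it.
; Box overlap sets an outline overlay material, and end overlap sets the door material as the overlay rather than clearing it.
; BeginPlay enables player 0 input, though no input events are defined here.
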(event OnComponentBeginOverlap(Box)
  (params (OverlappedComponent :type Primitive%20Component%20Object%20Reference) (OtherActor :type Actor%20Object%20Reference) (OtherComp :type Primitive%20Component%20Object%20Reference) (OtherBodyIndex :type Integer) (bFromSweep :type Boolean) (SweepResult :type Hit%20Result%20Structure%20%28by%20ref%29))
  (Rendering|Material|SetOverlayMaterial (Variables|Default|GetSK_Door_02_Anim) "/Game/Levels/Level1/Material/M_PP_Outline.M_PP_Outline" :!class /Script/Engine.MeshComponent))

(event OnComponentEndOverlap(Box)
  (params (OverlappedComponent :type Primitive%20Component%20Object%20Reference) (OtherActor :type Actor%20Object%20Reference) (OtherComp :type Primitive%20Component%20Object%20Reference) (OtherBodyIndex :type Integer))
  (Rendering|Material|SetOverlayMaterial (Variables|Default|GetSK_Door_02_Anim) "/Game/Levels/Level1/Material/M_Door_01.M_Door_01" :!class /Script/Engine.MeshComponent))

(event Collision|EventActorBeginOverlap
  (params (OtherActor :type Actor%20Object%20Reference)))

(event EventTick
  (params (DeltaSeconds :type Float%20%28single-precision%29)))

(event EventBeginPlay
  (Input|EnableInput (Game|GetPlayerController 0)))

(fn ConstructionScript)

(fn InteractDoor
  (bind _sk_door_02_anim (Variables|Default|GetSK_Door_02_Anim))
  (if (Variables|Default|GetIsOpened)
    (Components|Animation|PlayAnimation _sk_door_02_anim "/Game/Levels/Level1/Skeletal_Mesh/Door_01_Anim_Anim_ArmatureDoor_01_Door_01_Close.Door_01_Anim_Anim_ArmatureDoor_01_Door_01_Close" false)
    (Variables|Default|SetIsOpened false)
    (else
      (Components|Animation|PlayAnimation _sk_door_02_anim "/Game/Levels/Level1/Skeletal_Mesh/Door_01_Anim_Anim_ArmatureDoor_01_Door_01_Open.Door_01_Anim_Anim_ArmatureDoor_01_Door_01_Open" false)
      (Variables|Default|SetIsOpened true))))