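; Level 1 breaker panel actor that sets itself up as an objective with a randomly chosen breaker.
; On BeginPlay it sorts its child actors into a breaker array, an LED indicator and a gauge.
; SetRandomObjective flags a random breaker, stores ObjectiveBreaker from a separate random roll (possibly a different breaker), and prints debug states.
; The LED then turns red and the gauge needle gets a random low value.
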(event EventBeginPlay
  (for _array_element (Actor|GetComponentsByClass "/Script/Engine.ChildActorComponent")
    (bind _asbp_breaker_level_1 (Utilities|Casting|CastToBP_BreakerLevel1 (Variables|/Script/Engine.ChildActorComponent|GetChildActor _array_element))
      (:then
        (Utilities|IsValid _asbp_breaker_level_1
          (:Is%20Valid
            (Utilities|Array|Add (Variables|Default|GetBreakerArray) _asbp_breaker_level_1))))
      (:CastFailed
        (bind _asbp_ledindicator (Utilities|Casting|CastToBP_LEDIndicator (Variables|/Script/Engine.ChildActorComponent|GetChildActor _array_element))
          (:then
            (bind _output_get (Variables|Default|SetLEDIndicator _asbp_ledindicator))
            (Development|PrintString (Utilities|GetDisplayName _output_get)))
          (:CastFailed
            (bind _asbp_gauge (Utilities|Casting|CastToBP_Gauge (Variables|/Script/Engine.ChildActorComponent|GetChildActor _array_element)))
            (bind _output_get_2 (Variables|Default|SetGauge _asbp_gauge))
            (Development|PrintString (Utilities|GetDisplayName _output_get_2)))))))
  (CallFunction|SetRandomObjective)
  (Default|TurnRed (Variables|Default|GetLEDIndicator))
  (Default|TurnNeedle (Variables|Default|GetGauge) (Math|Random|RandomFloatinRange 0.1 0.2)))

(event Collision|EventActorBeginOverlap
  (params (OtherActor :type Actor%20Object%20Reference)))

(event EventTick
  (params (DeltaSeconds :type Float%20%28single-precision%29)))

(fn ConstructionScript)

(fn SetRandomObjective
  (bind _breakerarray (Variables|Default|GetBreakerArray))
  (bind _returnvalue (Utilities|Array|Length _breakerarray))
  (bind _returnvalue_2 (- _returnvalue 1))
  (bind _returnvalue_3 (Math|Random|RandomIntegerinRange 0 _returnvalue_2))
  (bind _output (Utilities|Array|Get(acopy) _breakerarray _returnvalue_3))
  (Variables|/Game/Levels/Level1/Blueprints/BP_BreakerLevel1.BP_BreakerLevel1_C|SetObjective _output true)
  (Variables|Default|SetObjectiveBreaker _output)
  (Variables|Default|SetPanelIsObjective true)
  (for _array_element _breakerarray
    (Development|PrintString (Utilities|String|Append (Utilities|GetDisplayName _array_element) (Utilities|String|ToString(Boolean) (Variables|/Game/Levels/Level1/Blueprints/BP_BreakerLevel1.BP_BreakerLevel1_C|GetObjective _array_element))) true true "(R=0.000000,G=0.660000,B=1.000000,A=1.000000)" 1e+01)))